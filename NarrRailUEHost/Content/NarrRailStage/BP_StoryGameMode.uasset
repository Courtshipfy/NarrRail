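; Game mode for a NarrRail story game that puts the WBP_Start widget on screen at BeginPlay.
; The rest of the graph is disconnected.
; One unused chain creates an NVL dialogue widget as presenter for a 蜗物语 session bound to the NarrRail player controller.
; Another, marked as the old method, builds a branching test dialogue in code with an Affinity variable, choices and conditional endings.
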(event EventBeginPlay
  (bind _returnvalue (UserInterface|CreateWidget "/Game/NarrRailStage/UI/WBP_Start.WBP_Start_C"))
  (UserInterface|Viewport|AddtoViewport _returnvalue 0))

(fn ConstructionScript)