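; BP_StoryController is a controller for NarrRail story playback that shows the mouse cursor and handles advance input.
; Left mouse and Space share one path: an unfinished typewriter effect completes immediately, while a finished one calls Next on the NarrRail session if it is Running.
; A missing session prints a red error pointing to BindNarrRailSession, checked only once the typewriter has completed.
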(event EventBeginPlay
  (Variables|Default|SetbShowMouseCursor true))

(event Input|MouseEvents|LeftMouseButton
  (params (Key :type Key%20Structure :default "None"))
  (bind _returnvalue (Class|NarrRailPlayerController|GetTypewriterController))
  (bind _returnvalue_2 (Class|NarrRailPlayerController|GetNarrRailSession))
  (:Pressed
    (Utilities|IsValid _returnvalue
      (:Is%20Valid
        (if (Class|NarrRailTypewriterController|IsCompleted _returnvalue)
          (Utilities|IsValid (Class|NarrRailPlayerController|GetNarrRailSession)
            (:Is%20Valid
              (if (Utilities|Enum|Equal(Enum) (Class|NarrRailStorySession|GetSessionState _returnvalue_2) "Running")
                (Class|NarrRailStorySession|Next _returnvalue_2)))
            (:Is%20Not%20Valid
              (Development|PrintString "Session is null, use BindNarrRailSession When Create session" true true "(R=1.000000,G=0.000000,B=0.000000,A=1.000000)")))
          (else
            (Class|NarrRailTypewriterController|CompleteImmediately _returnvalue)))))))

(event Input|KeyboardEvents|SpaceBar
  (params (Key :type Key%20Structure :default "None"))
  (bind _returnvalue (Class|NarrRailPlayerController|GetTypewriterController))
  (bind _returnvalue_2 (Class|NarrRailPlayerController|GetNarrRailSession))
  (:Pressed
    (Utilities|IsValid _returnvalue
      (:Is%20Valid
        (if (Class|NarrRailTypewriterController|IsCompleted _returnvalue)
          (Utilities|IsValid (Class|NarrRailPlayerController|GetNarrRailSession)
            (:Is%20Valid
              (if (Utilities|Enum|Equal(Enum) (Class|NarrRailStorySession|GetSessionState _returnvalue_2) "Running")
                (Class|NarrRailStorySession|Next _returnvalue_2)))
            (:Is%20Not%20Valid
              (Development|PrintString "Session is null, use BindNarrRailSession When Create session" true true "(R=1.000000,G=0.000000,B=0.000000,A=1.000000)")))
          (else
            (Class|NarrRailTypewriterController|CompleteImmediately _returnvalue)))))))

(fn ConstructionScript)