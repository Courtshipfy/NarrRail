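; Game mode for a NarrRail narrative sample that plays the Kiminoshiranai_narrrail story through an NVL-style dialogue UI.
; On BeginPlay it adds WBP_Dialogue_NVL to the viewport, creates a StorySession from the story asset, registers the widget as dialogue presenter and starts the session.
; Disconnected legacy nodes show the old approach of building a branching, affinity-based test story in code; they never run.
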(event EventBeginPlay
  (Utilities|FlowControl|Sequence
    (:then_0
      (bind _returnvalue (UserInterface|CreateWidget "/NarrRail/UI/NVL/WBP_Dialogue_NVL.WBP_Dialogue_NVL_C"))
      (UserInterface|Viewport|AddtoViewport _returnvalue 0))
    (:then_1
      (bind _returnvalue_2 (Class|NarrRailBlueprintLibrary|CreateStorySession "/Game/NarrRailSample/SampleTest_02/kiminoshiranai_narrrail.kiminoshiranai_narrrail"))
      (bind _output_get (Variables|Default|SetStorySession _returnvalue_2))
      (Utilities|IsValid _output_get
        (:Is%20Valid
          (Class|NarrRailStorySession|RegisterDialoguePresenter _output_get _returnvalue)
          (Class|NarrRailStorySession|Start _output_get "None"))))))

(fn ConstructionScript)