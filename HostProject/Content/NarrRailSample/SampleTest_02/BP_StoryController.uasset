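; BP_StoryController is a player controller for a NarrRail sample that lets the player advance a story session.
; It shows the mouse cursor on BeginPlay.
; Left mouse button and Space Bar share one path that gets the Storysession from BP_StoryGameMode and calls Next only while its state is Running.
; Each advance also prints a "Hello" debug string.
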(event EventBeginPlay
  (Variables|Default|SetbShowMouseCursor true))

(event Input|MouseEvents|LeftMouseButton
  (params (Key :type Key%20Structure :default "None"))
  (:Pressed
    (bind _asbp_story_game_mode (Utilities|Casting|CastToBP_StoryGameMode (Game|GetGameMode)))
    (if (Utilities|Enum|Equal(Enum) (Class|NarrRailStorySession|GetSessionState (Variables|/Game/NarrRailSample/SampleTest_02/BP_StoryGameMode.BP_StoryGameMode_C|Getstorysession _asbp_story_game_mode)) "Running")
      (Class|NarrRailStorySession|Next (Variables|/Game/NarrRailSample/SampleTest_02/BP_StoryGameMode.BP_StoryGameMode_C|Getstorysession _asbp_story_game_mode))
      (Development|PrintString "Hello"))))

(event Input|KeyboardEvents|SpaceBar
  (params (Key :type Key%20Structure :default "None"))
  (:Pressed
    (bind _asbp_story_game_mode (Utilities|Casting|CastToBP_StoryGameMode (Game|GetGameMode)))
    (if (Utilities|Enum|Equal(Enum) (Class|NarrRailStorySession|GetSessionState (Variables|/Game/NarrRailSample/SampleTest_02/BP_StoryGameMode.BP_StoryGameMode_C|Getstorysession _asbp_story_game_mode)) "Running")
      (Class|NarrRailStorySession|Next (Variables|/Game/NarrRailSample/SampleTest_02/BP_StoryGameMode.BP_StoryGameMode_C|Getstorysession _asbp_story_game_mode))
      (Development|PrintString "Hello"))))

(fn ConstructionScript)