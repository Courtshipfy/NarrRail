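; BP_NarrRailRunner is a sample Blueprint that runs a NarrRail story from its StoryAsset.
; On BeginPlay it constructs a NarrRailStorySession, initializes it with the asset and, on success, starts it with a start argument of None.
; Every Tick it prints the session's current node ID to show where the story is.
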(event EventBeginPlay
  (bind _returnvalue (Game|ConstructObjectfromClass "/Script/NarrRail.NarrRailStorySession"))
  (bind _output_get (Variables|Default|SetSession _returnvalue))
  (bind _returnvalue_2 (Class|NarrRailStorySession|Initialize _output_get (Variables|Default|GetStoryAsset)))
  (if (Utilities|Enum|Equal(Enum) (.code _returnvalue_2) "Success")
    (Class|NarrRailStorySession|Start _output_get "None")))

(event EventTick
  (params (DeltaSeconds :type Float%20%28single-precision%29))
  (Development|PrintString (Utilities|String|ToString(Name) (.nodeid (.OutNode (Class|NarrRailStorySession|GetCurrentNode (Variables|Default|GetSession)))))))

(fn ConstructionScript)