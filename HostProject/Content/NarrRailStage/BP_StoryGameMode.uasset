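; Game mode that boots a NarrRail visual-novel story session on BeginPlay.
; It adds an NVL dialogue widget to the viewport, creates a session from the 撫物語_narrrail story asset, registers the widget as presenter, binds the NarrRail player controller and starts the session.
; Disconnected legacy graph code builds a sample branching dialogue at runtime, using an Affinity variable and conditional edges, but never runs.
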(event EventBeginPlay
  (Utilities|FlowControl|Sequence
    (:then_0
      (bind _returnvalue (UserInterface|CreateWidget "/NarrRail/UI/NVL/WBP_Dialogue_NVL.WBP_Dialogue_NVL_C"))
      (UserInterface|Viewport|AddtoViewport _returnvalue 0))
    (:then_1
      (bind _returnvalue_2 (Class|NarrRailBlueprintLibrary|CreateStorySession "/Game/MonogatariStories/撫物語_narrrail.撫物語_narrrail"))
      (bind _output_get (Variables|Default|SetStorySession _returnvalue_2))
      (Utilities|IsValid _output_get
        (:Is%20Valid
          (Class|NarrRailStorySession|RegisterDialoguePresenter _output_get _returnvalue)
          (bind _asnarr_rail_player_controller (Utilities|Casting|CastToNarrRailPlayerController (Game|GetPlayerController 0)))
          (Class|NarrRailPlayerController|BindNarrRailSession _asnarr_rail_player_controller (Variables|Default|Getstorysession))
          (Class|NarrRailStorySession|Start _output_get "None"))))))

(fn ConstructionScript)